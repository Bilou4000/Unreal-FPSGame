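; Fire demon enemy for a first-person game, drawn as a Paper2D flipbook with eight-direction, Doom-style sprites.
; Each tick, dot products against the player direction pick the sprite and its rotation; only the front view enables timed projectiles aimed at the player.
; Pawn sensing stores the player and a seen flag, which this graph's firing ignores.
; Lethal damage stops movement, plays death and corpse flipbooks turned toward the player, then destroys the actor.
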(event OnSeePawn(PawnSensing)
  (params (Pawn :type Pawn%20Object%20Reference))
  (bind _asbp_fpscharacter (Utilities|Casting|CastToBP_FPSCharacter Pawn))
  (Variables|Default|Setplayer _asbp_fpscharacter)
  (Variables|Default|SetcanSeePlayer true))

(event EventBeginPlay
  (Variables|Default|SetcurrentHealth (Variables|Default|GetmaxHealth)))

(event EventTick
  (params (DeltaSeconds :type Float%20%28single-precision%29))
  (if (Variables|Default|GetisDead)
    ;[1 1 1] Death
    (Transformation|SetRelativeRotation (Variables|Default|GetPaperFlipbook) "0.000000,90.000000,0.000000" false false)
    (Transformation|SetRelativeLocation (Variables|Default|GetPaperFlipbook) "0.000000,0.000000,-60.000000" false false)
    (Transformation|SetActorRotation (Math|Rotator|MakeRotator 0.0 0.0 (.yaw (Math|Rotator|FindLookatRotation (Transformation|GetActorLocation) (Transformation|GetActorLocation (Game|GetPlayerCharacter 0))))))
    (else
      (CallFunction|EightDirectionSprite)
      (if (and (Variables|Default|GetisFacingForward) (Variables|Default|GetcanFire))
        ;[1 1 1] Shoot projectile
        (Transformation|SetWorldRotation (Variables|Default|GetSpawnProjectile) (Math|Rotator|MakeRotator 0.0 0.0 (.yaw (Math|Rotator|FindLookatRotation (Transformation|GetActorLocation) (Transformation|GetActorLocation (Game|GetPlayerCharacter 0))))) false false)
        (Game|SpawnActorfromClass "/Game/Blueprints/Projectile/BP_FireProjectile.BP_FireProjectile_C" (Transformation|GetWorldTransform (Variables|Default|GetSpawnProjectile)) "Undefined" "MultiplyWithRoot" 0 0)
        (Variables|Default|SetcanFire false)
        (Utilities|FlowControl|Delay (Variables|Default|GettimeBetweenProjectile))
        (Variables|Default|SetcanFire true)))))

(event Game|Damage|EventAnyDamage
  (params (Damage :type Float%20%28single-precision%29) (DamageType :type Damage%20Type%20Object%20Reference) (InstigatedBy :type Controller%20Object%20Reference) (DamageCauser :type Actor%20Object%20Reference))
  (bind _paperflipbook (Variables|Default|GetPaperFlipbook))
  ;[1 1 1] Get hurt
  (bind _output_get (Variables|Default|SetcurrentHealth (- (Variables|Default|GetcurrentHealth) Damage)))
  (if (<= _output_get 0.0)
    (Variables|Default|SetisDead true)
    ;[1 1 1] Die
    (Utilities|FlowControl|DoOnce false
      (:Completed
        (Components|Activation|Deactivate (Variables|Character|GetCharacterMovement))
        (Sprite|SetFlipbook _paperflipbook "/Game/Asset/Enemy/Firedemon/Death/FireDemonDeath.FireDemonDeath")
        (Utilities|FlowControl|Delay (Class|PaperFlipbookComponent|GetFlipbookLength _paperflipbook))
        (Sprite|SetFlipbook (Variables|Default|GetPaperFlipbook) "/Game/Asset/Enemy/Firedemon/Death/FireDemonDeadBody.FireDemonDeadBody")
        (Utilities|FlowControl|Delay 4.0)
        (Actor|DestroyActor)))))

(fn ConstructionScript)

(fn EightDirectionSprite
  (bind _returnvalue (Game|GetPlayerCharacter 0))
  (bind _self self)
  (bind _returnvalue_2 (Transformation|GetActorLocation _returnvalue))
  (bind _returnvalue_3 (Transformation|GetActorLocation _self))
  (bind _returnvalue_4 (- _returnvalue_2 _returnvalue_3))
  (bind _returnvalue_5 (Math|Vector|Normalize _returnvalue_4))
  (Variables|Default|Setdegrees (Class|KismetMathLibrary|DegAcos (Math|Vector|DotProduct (Transformation|GetActorForwardVector) _returnvalue_5)))
  (if (< (Math|Vector|DotProduct (Transformation|GetActorRightVector) _returnvalue_5) 0.0)
    (Math|Float|CompareFloat (Variables|Default|Getdegrees) 1.8e+02
      (:>
        ;[1 1 1] Attack player
        (Transformation|SetRelativeRotation (Variables|Default|GetPaperFlipbook) "0.000000,-90.000000,0.000000" false false :!label _label) ; front
        (Sprite|SetFlipbook (Variables|Default|GetPaperFlipbook) (Utilities|Array|Get(acopy) (Variables|Default|GetflipbooksIdle)))
        (Variables|Default|SetisFacingForward true))
      (:==
        (goto _label))
      (:<
        (Math|Float|CompareFloat (Variables|Default|Getdegrees) 135.0
          (:>
            (Transformation|SetRelativeRotation (Variables|Default|GetPaperFlipbook) "0.000000,135.000000,0.000000" false false :!label _label_2) ; back left
            (Sprite|SetFlipbook (Variables|Default|GetPaperFlipbook) (Utilities|Array|Get(acopy) (Variables|Default|GetflipbooksIdle) 3))
            (Variables|Default|SetisFacingForward false))
          (:==
            (goto _label_2))
          (:<
            (Math|Float|CompareFloat (Variables|Default|Getdegrees) 9e+01
              (:>
                (Transformation|SetRelativeRotation (Variables|Default|GetPaperFlipbook) "0.000000,180.000000,0.000000" false false :!label _label_3) ; left
                (Sprite|SetFlipbook (Variables|Default|GetPaperFlipbook) (Utilities|Array|Get(acopy) (Variables|Default|GetflipbooksIdle) 2))
                (Variables|Default|SetisFacingForward false))
              (:==
                (goto _label_3))
              (:<
                (Math|Float|CompareFloat (Variables|Default|Getdegrees) 45.0
                  (:>
                    _)
                  (:==
                    _)
                  (:<
                    (goto _label)))
                (Transformation|SetRelativeRotation (Variables|Default|GetPaperFlipbook) "0.000000,45.000000,0.000000" false false) ; front right
                (Sprite|SetFlipbook (Variables|Default|GetPaperFlipbook) (Utilities|Array|Get(acopy) (Variables|Default|GetflipbooksIdle) 1))
                (Variables|Default|SetisFacingForward false)))))))
    (else
      (Math|Float|CompareFloat (Variables|Default|Getdegrees) 1.8e+02
        (:>
          (Transformation|SetRelativeRotation (Variables|Default|GetPaperFlipbook) "0.000000,-45.000000,0.000000" false false :!label _label_4) ; front
          (Sprite|SetFlipbook (Variables|Default|GetPaperFlipbook) (Utilities|Array|Get(acopy) (Variables|Default|GetflipbooksIdle) 7))
          (Variables|Default|SetisFacingForward false))
        (:==
          (goto _label_4))
        (:<
          (Math|Float|CompareFloat (Variables|Default|Getdegrees) 135.0
            (:>
              (Transformation|SetRelativeRotation (Variables|Default|GetPaperFlipbook) "0.000000,90.000000,0.000000" false false :!label _label_5) ; back left
              (Sprite|SetFlipbook (Variables|Default|GetPaperFlipbook) (Utilities|Array|Get(acopy) (Variables|Default|GetflipbooksIdle) 4))
              (Variables|Default|SetisFacingForward false))
            (:==
              (goto _label_5))
            (:<
              (Math|Float|CompareFloat (Variables|Default|Getdegrees) 9e+01
                (:>
                  (Transformation|SetRelativeRotation (Variables|Default|GetPaperFlipbook) "0.000000,45.000000,0.000000" false false :!label _label_6) ; left
                  (Sprite|SetFlipbook (Variables|Default|GetPaperFlipbook) (Utilities|Array|Get(acopy) (Variables|Default|GetflipbooksIdle) 5))
                  (Variables|Default|SetisFacingForward false))
                (:==
                  (goto _label_6))
                (:<
                  (Math|Float|CompareFloat (Variables|Default|Getdegrees) 45.0
                    (:>
                      _)
                    (:==
                      _)
                    (:<
                      (goto _label_4)))
                  (Transformation|SetRelativeRotation (Variables|Default|GetPaperFlipbook) "0, 0, 0" false false) ; front right
                  (Sprite|SetFlipbook (Variables|Default|GetPaperFlipbook) (Utilities|Array|Get(acopy) (Variables|Default|GetflipbooksIdle) 6))
                  (Variables|Default|SetisFacingForward false))))))))))