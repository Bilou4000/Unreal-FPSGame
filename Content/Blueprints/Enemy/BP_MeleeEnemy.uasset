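; Melee enemy for a first-person game, drawn with Paper2D flipbooks that swap for move, attack, hurt and death states.
; Pawn sensing sets the player as target, starting per-tick yaw facing and AI MoveTo.
; Arrival plays the attack flipbook, then damages the player without rechecking range; GetMeleeRange is never called here.
; Damage lowers health, triggering a hurt flipbook or a one-time death sequence that leaves a corpse briefly before destruction.
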(event OnSeePawn(PawnSensing)
  (params (Pawn :type Pawn%20Object%20Reference))
  ;[1 1 1] Move Toward Player if in sight
  (bind _asbp_fpscharacter (Utilities|Casting|CastToBP_FPSCharacter Pawn))
  (Variables|Default|SetPlayer _asbp_fpscharacter)
  (Variables|Default|SetcanSeePlayer true)
  (if (> (Variables|Default|GetcurrentHealth) 0.0)
    (AI|AIMoveTo self (Math|Vector|MakeVector 0.0 0.0 0.0) (Variables|Default|GetPlayer) (Variables|Default|GetstopRadius) false
      (:then
        (if (not (Variables|Default|GetisHurt))
          (Sprite|SetFlipbook (Variables|Default|GetPaperFlipbook) "/Game/Asset/Enemy/MeleeEnemy/Movement/MeleeMove.MeleeMove")))
      (:OnSuccess
        ;[1 1 1] Attack Player
        (bind _lenghtofanim (CallFunction|MeleeAttackAnim self))
        (Utilities|FlowControl|Delay _lenghtofanim)
        (CallFunction|DamagePlayer self)))))

(event EventBeginPlay
  (Variables|Default|SetcurrentHealth (Variables|Default|GetmaxHealth)))

(event EventTick
  (params (DeltaSeconds :type Float%20%28single-precision%29))
  ;[1 1 1] Rotate Toward Player if in sight
  (if (Variables|Default|GetcanSeePlayer)
    (Transformation|SetActorRotation (Math|Rotator|MakeRotator 0.0 0.0 (.yaw (Math|Rotator|FindLookatRotation (Transformation|GetActorLocation) (Transformation|GetActorLocation (Variables|Default|GetPlayer))))))))

(event Game|Damage|EventAnyDamage
  (params (Damage :type Float%20%28single-precision%29) (DamageType :type Damage%20Type%20Object%20Reference) (InstigatedBy :type Controller%20Object%20Reference) (DamageCauser :type Actor%20Object%20Reference))
  (bind _paperflipbook (Variables|Default|GetPaperFlipbook))
  (bind _paperflipbook_2 (Variables|Default|GetPaperFlipbook))
  ;[1 1 1] Get hurt
  (bind _output_get (Variables|Default|SetcurrentHealth (- (Variables|Default|GetcurrentHealth) Damage)))
  (if (<= _output_get 0.0)
    ;[1 1 1] Die
    (Utilities|FlowControl|DoOnce false
      (:Completed
        (Components|Activation|Deactivate (Variables|Character|GetCharacterMovement))
        (Sprite|SetFlipbook _paperflipbook "/Game/Asset/Enemy/MeleeEnemy/Death/EnemyMeleeDeath.EnemyMeleeDeath")
        (Utilities|FlowControl|Delay (Class|PaperFlipbookComponent|GetFlipbookLength _paperflipbook))
        (Sprite|SetFlipbook (Variables|Default|GetPaperFlipbook) "/Game/Asset/Enemy/MeleeEnemy/Death/DeadBody.DeadBody")
        (Transformation|SetRelativeLocation (Variables|Default|GetPaperFlipbook) "0.000000,0.000000,-60.000000" false false)
        (Utilities|FlowControl|Delay 4.0)
        (Actor|DestroyActor)))
    (else
      ;[1 1 1] Hurt Anim
      (Variables|Default|SetisHurt true)
      (Transformation|SetWorldRotation (Variables|Character|GetMesh) (Math|Rotator|MakeRotator 0.0 0.0 (.yaw (Math|Rotator|FindLookatRotation (Transformation|GetActorLocation) (Transformation|GetActorLocation (Game|GetPlayerCharacter 0))))) false false)
      (Sprite|SetFlipbook _paperflipbook_2 "/Game/Asset/Enemy/MeleeEnemy/Death/MeleeHurt.MeleeHurt")
      (Utilities|FlowControl|Delay (Class|PaperFlipbookComponent|GetFlipbookLength _paperflipbook_2))
      (Variables|Default|SetisHurt false))))

(fn ConstructionScript)

(fn GetMeleeRange
  ;[1 1 1] Check if enemy is in melee range
  (if (and (< (Math|Vector|Distance(Vector) (Transformation|GetActorLocation (Game|GetPlayerCharacter 0)) (Transformation|GetActorLocation self)) (Variables|Default|GetmeleeDistance)) (Variables|Default|GetcanSeePlayer))
    (Variables|Default|SetcanAttack true)
    (else
      (Variables|Default|SetcanAttack false))))

(fn MeleeAttackAnim
  (bind _paperflipbook (Variables|Default|GetPaperFlipbook))
  (if (> (Variables|Default|GetcurrentHealth) 0.0)
    (Sprite|SetFlipbook _paperflipbook "/Game/Asset/Enemy/MeleeEnemy/Attack/MeleeAttack.MeleeAttack")
    (return (Class|PaperFlipbookComponent|GetFlipbookLength _paperflipbook))))

(fn DamagePlayer
  (if (> (Variables|Default|GetcurrentHealth) 0.0)
    (Default|OnTakeAnyDamageEvent (Variables|Default|GetPlayer) 0 1.0)
    (Sprite|SetFlipbook (Variables|Default|GetPaperFlipbook) "/Game/Asset/Enemy/MeleeEnemy/Idle/Melee_Forward.Melee_Forward")))