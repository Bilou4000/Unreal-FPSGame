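; Shotgun weapon Blueprint that fires and plays a 2D flipbook shooting animation.
; ShootWeapon passes a DoOnce gate, calls FireWeapon (defined outside this file) and switches WeaponFlipbook to the fire animation.
; After a delay equal to that flipbook's length, it restores the idle flipbook and calls ResetWeapon to reopen the gate, so the animation length sets the fire rate.
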(event Custom|ResetWeapon
  (bind _weaponflipbook (Variables|Default|GetWeaponFlipbook))
  (Utilities|FlowControl|DoOnce false) ; enters at Reset
)

(event EventBeginPlay
  (|CallParentFunction) ; This node is disabled and will not be called.\nDrag off pins to build functionality.
)

(event Collision|EventActorBeginOverlap
  (params (OtherActor :type Actor%20Object%20Reference))
  (|CallParentFunction OtherActor) ; This node is disabled and will not be called.\nDrag off pins to build functionality.
)

(event EventTick
  (params (DeltaSeconds :type Float%20%28single-precision%29))
  (|CallParentFunction DeltaSeconds) ; This node is disabled and will not be called.\nDrag off pins to build functionality.
)

(event EventShootWeapon
  (bind _weaponflipbook (Variables|Default|GetWeaponFlipbook))
  (Utilities|FlowControl|DoOnce false
    (:Completed
      (CallFunction|FireWeapon)
      (Sprite|SetFlipbook _weaponflipbook "/Game/Asset/Weapon/Sprites/Weapons/Shotgun/ShotgunFire.ShotgunFire")
      (Utilities|FlowControl|Delay (Class|PaperFlipbookComponent|GetFlipbookLength _weaponflipbook))
      (Sprite|SetFlipbook (Variables|Default|GetWeaponFlipbook) "/Game/Asset/Weapon/Sprites/Weapons/Shotgun/ShotgunIdle.ShotgunIdle")
      (CallFunction|ResetWeapon))))

(fn ConstructionScript
  (|CallParentFunction))