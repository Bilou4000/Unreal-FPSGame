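; BP_BaseWeapon is a base weapon Blueprint that provides hitscan firing.
; FireWeapon traces from the Linetrace component along its forward vector against static, dynamic and pawn objects, ignoring itself and the player character, then applies WeaponDamage to the hit actor.
; The trace draws debug lines for a duration.
; ShootWeapon and StopShooting are empty events, and nothing in this Blueprint calls FireWeapon.
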(event Custom|ShootWeapon)

(event Custom|StopShooting)

(fn ConstructionScript)

(fn FireWeapon
  (bind _linetrace (Variables|Default|GetLinetrace))
  (bind _returnvalue (Transformation|GetWorldLocation _linetrace))
  (bind (_outhit _returnvalue_2) (Collision|LineTraceForObjects _returnvalue (+ _returnvalue (* (Math|Vector|GetForwardVector (Transformation|GetWorldRotation (Variables|Default|GetLinetrace))) (Variables|Default|GetlineTraceDistance))) (Utilities|Array|MakeArray "ObjectTypeQuery1" "ObjectTypeQuery2" "ObjectTypeQuery3") false (Utilities|Array|MakeArray self (Game|GetPlayerCharacter 0)) "ForDuration"))
  (if _returnvalue_2
    (Game|Damage|ApplyDamage (.HitActor (Collision|BreakHitResult _outhit)) (Variables|Default|GetweaponDamage) 0 0)))