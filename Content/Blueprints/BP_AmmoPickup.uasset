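; An ammo pickup that refills the current weapon of BP_FPSCharacter when a Player-tagged actor overlaps its box collision.
; It finds the character with GetActorOfClass rather than using the overlapping actor, then reads its ammo arrays at the current weapon index.
; Below max, it adds a fixed amount or sets ammo to max, though the headroom check uses a larger amount than it adds, then destroys itself.
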(event OnComponentBeginOverlap(BoxCollision)
  (params (OverlappedComponent :type Primitive%20Component%20Object%20Reference) (OtherActor :type Actor%20Object%20Reference) (OtherComp :type Primitive%20Component%20Object%20Reference) (OtherBodyIndex :type Integer) (bFromSweep :type Boolean) (SweepResult :type Hit%20Result%20Structure%20%28by%20ref%29))
  (if (Actor|ActorHasTag OtherActor "Player")
    (bind _returnvalue (Actor|GetActorOfClass "/Game/FirstPerson/Blueprints/BP_FPSCharacter.BP_FPSCharacter_C"))
    (Variables|Default|SetcurrentWeaponAmmo (Utilities|Array|Get(acopy) (Variables|/Game/FirstPerson/Blueprints/BP_FPSCharacter.BP_FPSCharacter_C|GetweaponAmmo _returnvalue) (Variables|/Game/FirstPerson/Blueprints/BP_FPSCharacter.BP_FPSCharacter_C|GetindexWeapon _returnvalue)))
    (if (< (Utilities|Array|Get(acopy) (Variables|/Game/FirstPerson/Blueprints/BP_FPSCharacter.BP_FPSCharacter_C|GetweaponAmmo _returnvalue) (Variables|/Game/FirstPerson/Blueprints/BP_FPSCharacter.BP_FPSCharacter_C|GetindexWeapon _returnvalue)) (Utilities|Array|Get(acopy) (Variables|/Game/FirstPerson/Blueprints/BP_FPSCharacter.BP_FPSCharacter_C|GetweaponAmmoMax _returnvalue) (Variables|/Game/FirstPerson/Blueprints/BP_FPSCharacter.BP_FPSCharacter_C|GetindexWeapon _returnvalue)))
      (if (<= (+ (Variables|Default|GetcurrentWeaponAmmo) 5.0) (Utilities|Array|Get(acopy) (Variables|/Game/FirstPerson/Blueprints/BP_FPSCharacter.BP_FPSCharacter_C|GetweaponAmmoMax _returnvalue) (Variables|/Game/FirstPerson/Blueprints/BP_FPSCharacter.BP_FPSCharacter_C|GetindexWeapon _returnvalue)))
        (Utilities|Array|SetArrayElem (Variables|/Game/FirstPerson/Blueprints/BP_FPSCharacter.BP_FPSCharacter_C|GetweaponAmmo _returnvalue) (Variables|/Game/FirstPerson/Blueprints/BP_FPSCharacter.BP_FPSCharacter_C|GetindexWeapon _returnvalue) (+ (Variables|Default|GetcurrentWeaponAmmo) 3.0))
        (Actor|DestroyActor)
        (else
          (bind _output_get (Variables|Default|SetcurrentWeaponAmmo (Utilities|Array|Get(acopy) (Variables|/Game/FirstPerson/Blueprints/BP_FPSCharacter.BP_FPSCharacter_C|GetweaponAmmoMax _returnvalue) (Variables|/Game/FirstPerson/Blueprints/BP_FPSCharacter.BP_FPSCharacter_C|GetindexWeapon _returnvalue))))
          (Utilities|Array|SetArrayElem (Variables|/Game/FirstPerson/Blueprints/BP_FPSCharacter.BP_FPSCharacter_C|GetweaponAmmo _returnvalue) (Variables|/Game/FirstPerson/Blueprints/BP_FPSCharacter.BP_FPSCharacter_C|GetindexWeapon _returnvalue) _output_get)
          (Actor|DestroyActor))))))

(event EventBeginPlay)

(event Collision|EventActorBeginOverlap
  (params (OtherActor :type Actor%20Object%20Reference)))

(event EventTick
  (params (DeltaSeconds :type Float%20%28single-precision%29)))

(fn ConstructionScript)